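; BP_Axe is a thrown axe projectile that spins in flight and stops dead when its head meets a surface.
; Each tick, a one-unit Visibility line trace runs from AxeHead along world X, with debug drawing left on.
; The first blocking hit passes a DoOnce that halts ProjectileMovement, zeroes the RotatingMovement rate and removes projectile gravity, leaving the axe fixed in place.
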(event EventTick
  (params (DeltaSeconds :type Float%20%28single-precision%29))
  (bind _axehead (Variables|Default|GetAxeHead))
  (bind _projectilemovement (Variables|Default|GetProjectileMovement))
  (bind _returnvalue (Transformation|GetWorldLocation _axehead))
  (bind _outhit (Collision|LineTraceByChannel (Transformation|GetWorldLocation _axehead) (Math|Vector|MakeVector (+ (.x _returnvalue) 1.0) (.y _returnvalue) (.z _returnvalue)) "TraceTypeQuery1" false 0 "ForDuration"))
  (if (.bBlockingHit (Collision|BreakHitResult _outhit))
    (Utilities|FlowControl|DoOnce false
      (:Completed
        (Components|Movement|StopMovementImmediately _projectilemovement)
        (Variables|/Script/Engine.RotatingMovementComponent|SetRotationRate (Variables|Default|GetRotatingMovement) "0, 0, 0")
        (Variables|/Script/Engine.ProjectileMovementComponent|SetProjectileGravityScale _projectilemovement 0.0)))))

(fn ConstructionScript)